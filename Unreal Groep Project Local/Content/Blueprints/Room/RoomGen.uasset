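; RoomGen is an Actor Blueprint that builds a square, tile-based room in its Construction Script.
; A nested loop over MaxRoomSize places each cell at its index times TileSize as an instance on the CornerWall, Wall or Floor component.
; Corner and wall yaw comes branchlessly from summing edge-test booleans cast to int and multiplied by angles.
; The event graph holds only disabled default events.
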(event EventBeginPlay)

(event Collision|EventActorBeginOverlap
  (params (OtherActor :type Actor%20Object%20Reference)))

(event EventTick
  (params (DeltaSeconds :type Float%20%28single-precision%29)))

(fn ConstructionScript
  (bind _maxroomsize (Variables|Default|GetMaxRoomSize))
  (bind _tilesize (Variables|Default|GetTileSize))
  (bind _maxroomsize_2 (Variables|Default|GetMaxRoomSize))
  (bind _returnvalue (- _maxroomsize_2 0))
  (for _index (range 0 _maxroomsize)
    (bind _output_get (Variables|Default|SetIndexX _index))
    (for _index_2 (range 0 _maxroomsize)
      (bind _output_get_2 (Variables|Default|SetIndexY _index_2))
      (if (Math|Boolean|ORBoolean (and (== _output_get _returnvalue) (== _output_get_2 _returnvalue)) (and (== _output_get 0) (== _output_get_2 0)) (and (== _output_get _returnvalue) (== _output_get_2 0)) (and (== _output_get 0) (== _output_get_2 _returnvalue)))
        ;[1 1 1] Create corner piece instance
        (Components|InstancedStaticMesh|AddInstance (Variables|Default|GetCornerWall) (Math|Transform|MakeTransform (Math|Vector|MakeVector (Math|Conversions|ToFloat(Integer) (* _output_get _tilesize)) (Math|Conversions|ToFloat(Integer) (* _tilesize _output_get_2)) 0.0) (Math|Rotator|MakeRotator 0.0 0.0 (Math|Conversions|ToFloat(Integer) (+ (+ (* (Math|Conversions|ToInteger(Boolean) (and (== _output_get _returnvalue) (== _output_get_2 _returnvalue))) 270) (* (Math|Conversions|ToInteger(Boolean) (and (== _output_get 0) (== _output_get_2 0))) 90) (* (Math|Conversions|ToInteger(Boolean) (and (== _output_get _returnvalue) (== _output_get_2 0))) 180) (* (Math|Conversions|ToInteger(Boolean) (and (== _output_get 0) (== _output_get_2 _returnvalue))) 0)) 0)))))
        (elif (Math|Boolean|ORBoolean (== _output_get _returnvalue) (== _output_get 0) (== _output_get_2 _returnvalue) (== _output_get_2 0))
          ;[1 1 1] Create wall instance + rotation
          (Components|InstancedStaticMesh|AddInstance (Variables|Default|GetWall) (Math|Transform|MakeTransform (Math|Vector|MakeVector (Math|Conversions|ToFloat(Integer) (* _output_get _tilesize)) (Math|Conversions|ToFloat(Integer) (* _tilesize _output_get_2)) 0.0) (Math|Rotator|MakeRotator 0.0 0.0 (Math|Conversions|ToFloat(Integer) (+ (+ (* (Math|Conversions|ToInteger(Boolean) (== _output_get _returnvalue)) -90) (* (Math|Conversions|ToInteger(Boolean) (== _output_get 0)) 90) (* (Math|Conversions|ToInteger(Boolean) (== _output_get_2 _returnvalue)) 0) (* (Math|Conversions|ToInteger(Boolean) (== _output_get_2 0)) 180)) 0)))))
          (else
            ;[1 1 1] Create floor instance
            (Components|InstancedStaticMesh|AddInstance (Variables|Default|GetFloor) (Math|Conversions|ToTransform(Vector) (Math|Vector|MakeVector (Math|Conversions|ToFloat(Integer) (* _output_get _tilesize)) (Math|Conversions|ToFloat(Integer) (* _tilesize _output_get_2)) 0.0)))))))))