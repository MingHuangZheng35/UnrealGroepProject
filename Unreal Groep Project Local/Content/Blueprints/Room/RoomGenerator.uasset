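; RoomGenerator builds a square, tiled room from static mesh pieces at BeginPlay.
; Nested loops walk a RoomSize grid at 200-unit spacing, spawning a StaticMeshActor per cell with a corner, wall or floor mesh chosen by edge position.
; An outer loop offsets rooms along X but runs only once.
; Piece rotation is unfinished: spawn transforms set location only, and the rotation logic is unconnected.
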(event EventBeginPlay
  (bind _roomsize (Variables|Default|GetRoomSize))
  (bind _returnvalue (- _roomsize 1))
  (for _index (range 0 0)
    ;[1 1 1] Room
    (for _index_2 (range 0 _returnvalue)
      (for _index_3 (range 0 _returnvalue)
        (Utilities|FlowControl|Sequence
          (:then_0
            (Variables|Default|SetRotation "0, 0, 0"))
          (:then_1
            ;;[1 1 1] Choose the piece to place
            (if (or (Math|Boolean|ORBoolean (and (== _index_3 0) (== _index_2 0)) (and (== _index_3 0) (== _index_2 _returnvalue)) (and (== _index_3 _returnvalue) (== _index_2 0)) (and (== _index_3 _returnvalue) (== _index_2 _returnvalue))) (or (or (== _index_3 0) (== _index_3 _returnvalue)) (or (== _index_2 0) (== _index_2 _returnvalue))))
              (Utilities|FlowControl|Sequence
                (:then_0
                  ;;[1 1 1] Rotation
                  (Utilities|FlowControl|Sequence))
                (:then_1
                  (if (and (Math|Boolean|ORBoolean (and (== _index_3 0) (== _index_2 0)) (and (== _index_3 0) (== _index_2 _returnvalue)) (and (== _index_3 _returnvalue) (== _index_2 0)) (and (== _index_3 _returnvalue) (== _index_2 _returnvalue))) (or (Math|Boolean|ORBoolean (and (== _index_3 0) (== _index_2 0)) (and (== _index_3 0) (== _index_2 _returnvalue)) (and (== _index_3 _returnvalue) (== _index_2 0)) (and (== _index_3 _returnvalue) (== _index_2 _returnvalue))) (or (or (== _index_3 0) (== _index_3 _returnvalue)) (or (== _index_2 0) (== _index_2 _returnvalue)))))
                    ;;[1 1 1] Corner Piece
                    (bind _returnvalue_2 (Game|SpawnActorfromClass "/Script/Engine.StaticMeshActor" (Math|Transform|MakeTransform (Math|Vector|MakeVector (+ (Math|Conversions|ToFloat(Integer) (* _index_3 200)) (.X (Math|Vector|BreakVector (Math|Vector|MakeVector (* (Math|Conversions|ToFloat(Integer) _index) (* (Math|Conversions|ToFloat(Integer) _returnvalue) 2e+02)) 0.0 0.0)))) (+ (Math|Conversions|ToFloat(Integer) (* _index_2 200)) (.Y (Math|Vector|BreakVector (Math|Vector|MakeVector (* (Math|Conversions|ToFloat(Integer) _index) (* (Math|Conversions|ToFloat(Integer) _returnvalue) 2e+02)) 0.0 0.0)))) (.Z (Math|Vector|BreakVector (Math|Vector|MakeVector (* (Math|Conversions|ToFloat(Integer) _index) (* (Math|Conversions|ToFloat(Integer) _returnvalue) 2e+02)) 0.0 0.0))))) "Undefined" 0 0))
                    (Components|StaticMesh|SetStaticMesh (Variables|/Script/Engine.StaticMeshActor|GetStaticMeshComponent _returnvalue_2) "/Game/Models/Room/Room_Corner.Room_Corner")
                    (else
                      ;;[1 1 1] Wall
                      (bind _returnvalue_3 (Game|SpawnActorfromClass "/Script/Engine.StaticMeshActor" (Math|Transform|MakeTransform (Math|Vector|MakeVector (+ (Math|Conversions|ToFloat(Integer) (* _index_3 200)) (.X (Math|Vector|BreakVector (Math|Vector|MakeVector (* (Math|Conversions|ToFloat(Integer) _index) (* (Math|Conversions|ToFloat(Integer) _returnvalue) 2e+02)) 0.0 0.0)))) (+ (Math|Conversions|ToFloat(Integer) (* _index_2 200)) (.Y (Math|Vector|BreakVector (Math|Vector|MakeVector (* (Math|Conversions|ToFloat(Integer) _index) (* (Math|Conversions|ToFloat(Integer) _returnvalue) 2e+02)) 0.0 0.0)))) (.Z (Math|Vector|BreakVector (Math|Vector|MakeVector (* (Math|Conversions|ToFloat(Integer) _index) (* (Math|Conversions|ToFloat(Integer) _returnvalue) 2e+02)) 0.0 0.0))))) "Undefined" 0 0))
                      (Components|StaticMesh|SetStaticMesh (Variables|/Script/Engine.StaticMeshActor|GetStaticMeshComponent _returnvalue_3) "/Game/Models/Room/Room_Wall.Room_Wall")))))
              (else
                ;;[1 1 1] Flooring
                (bind _returnvalue_4 (Game|SpawnActorfromClass "/Script/Engine.StaticMeshActor" (Math|Transform|MakeTransform (Math|Vector|MakeVector (+ (Math|Conversions|ToFloat(Integer) (* _index_3 200)) (.X (Math|Vector|BreakVector (Math|Vector|MakeVector (* (Math|Conversions|ToFloat(Integer) _index) (* (Math|Conversions|ToFloat(Integer) _returnvalue) 2e+02)) 0.0 0.0)))) (+ (Math|Conversions|ToFloat(Integer) (* _index_2 200)) (.Y (Math|Vector|BreakVector (Math|Vector|MakeVector (* (Math|Conversions|ToFloat(Integer) _index) (* (Math|Conversions|ToFloat(Integer) _returnvalue) 2e+02)) 0.0 0.0)))) (.Z (Math|Vector|BreakVector (Math|Vector|MakeVector (* (Math|Conversions|ToFloat(Integer) _index) (* (Math|Conversions|ToFloat(Integer) _returnvalue) 2e+02)) 0.0 0.0))))) "Undefined" 0 0))
                (Components|StaticMesh|SetStaticMesh (Variables|/Script/Engine.StaticMeshActor|GetStaticMeshComponent _returnvalue_4) "/Game/Models/Room/room_empty.room_empty")))))))))

(event EventTick
  (params (DeltaSeconds :type Float%20%28single-precision%29)))